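; BP_Enviroment2 is an environment segment for the runner game that fills itself with randomly chosen rocks.
; Its construction script runs SpawnRocks, which rolls separately for each hand-placed SP point to add one of several child actor components or leave it empty.
; Any overlap with its Box asks BP_RunnerGameMode to extend the environment.
; GetAttachPoint exposes the Arrow's world transform as an attach point.
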(event `self.Box.OnComponentBeginOverlap`
  (params (OverlappedComponent :type "PrimitiveComponent Object Reference") (OtherActor :type "Actor Object Reference") (OtherComp :type "PrimitiveComponent Object Reference") (OtherBodyIndex :type Integer) (bFromSweep :type Boolean) (SweepResult :type "HitResult Structure (by ref)"))
  ; Extend Enviroment
  (bind _asbp_runner_game_mode (cast `/Game/Runner/Blueprints/BP_RunnerGameMode` (`GameplayStatics.GetGameMode`)))
  (`/Game/Runner/Blueprints/BP_RunnerGameMode.Extend Enviroment` _asbp_runner_game_mode))

(fn `Get AttachPoint`
  (returns (ReturnValue :type "Transform Structure"))
  (return (`SceneComponent.K2_GetComponentToWorld` (`self.Arrow`))))

(fn `Spawn rocks`
  (bind _returnvalue (`SceneComponent.GetRelativeTransform` (`self.SP2`)))
  (bind _returnvalue_2 (`SceneComponent.GetRelativeTransform` (`self.SP6`)))
  (bind _returnvalue_3 (`SceneComponent.GetRelativeTransform` (`self.SP7`)))
  (bind _returnvalue_4 (`SceneComponent.GetRelativeTransform` (`self.SP8`)))
  (bind _returnvalue_5 (`SceneComponent.GetRelativeTransform` (`self.SP9`)))
  (bind _returnvalue_6 (`SceneComponent.GetRelativeTransform` (`self.SP3`)))
  (bind _returnvalue_7 (`SceneComponent.GetRelativeTransform` (`self.SP10`)))
  (bind _returnvalue_8 (`SceneComponent.GetRelativeTransform` (`self.SP11`)))
  (bind _returnvalue_9 (`SceneComponent.GetRelativeTransform` (`self.SP12`)))
  (bind _returnvalue_10 (`SceneComponent.GetRelativeTransform` (`self.SP25`)))
  (bind _returnvalue_11 (`SceneComponent.GetRelativeTransform` (`self.SP1`)))
  (bind _returnvalue_12 (`SceneComponent.GetRelativeTransform` (`self.SP4`)))
  (bind _returnvalue_13 (`SceneComponent.GetRelativeTransform` (`self.SP13`)))
  (bind _returnvalue_14 (`SceneComponent.GetRelativeTransform` (`self.SP14`)))
  (bind _returnvalue_15 (`SceneComponent.GetRelativeTransform` (`self.SP15`)))
  (bind _returnvalue_16 (`SceneComponent.GetRelativeTransform` (`self.SP16`)))
  (bind _returnvalue_17 (`SceneComponent.GetRelativeTransform` (`self.SP17`)))
  (bind _returnvalue_18 (`SceneComponent.GetRelativeTransform` (`self.SP18`)))
  (bind _returnvalue_19 (`SceneComponent.GetRelativeTransform` (`self.SP19`)))
  (bind _returnvalue_20 (`SceneComponent.GetRelativeTransform` (`self.SP20`)))
  (bind _returnvalue_21 (`SceneComponent.GetRelativeTransform` (`self.SP21`)))
  (bind _returnvalue_22 (`SceneComponent.GetRelativeTransform` (`self.SP22`)))
  (bind _returnvalue_23 (`SceneComponent.GetRelativeTransform` (`self.SP24`)))
  (bind _returnvalue_24 (`SceneComponent.GetRelativeTransform` (`self.SP5`)))
  (`|ExecutionSequence`
    (:`then_0`
      (switch `int` (`KismetMathLibrary.RandomIntegerInRange` 0 8)
        (:`0`
          (`AddComponent|NODE_AddChildActorComponent-210` :`RelativeTransform` _returnvalue_11))
        (:`1`
          (`AddComponent|NODE_AddChildActorComponent-211` :`RelativeTransform` _returnvalue_11))
        (:`2`
          (`AddComponent|NODE_AddChildActorComponent-212` :`RelativeTransform` _returnvalue_11))
        (:`3`
          (`AddComponent|NODE_AddChildActorComponent-213` :`RelativeTransform` _returnvalue_11))
        (:`4`
          (`AddComponent|NODE_AddChildActorComponent-214` :`RelativeTransform` _returnvalue_11))
        (:`5`
          (`AddComponent|NODE_AddChildActorComponent-215` :`RelativeTransform` _returnvalue_11))
        (:`6`
          (`AddComponent|NODE_AddChildActorComponent-216` :`RelativeTransform` _returnvalue_11))
        (:`7`
          (`AddComponent|NODE_AddChildActorComponent-217` :`RelativeTransform` _returnvalue_11))))
    (:`then_1`
      ; SP2
      (switch `int` (`KismetMathLibrary.RandomIntegerInRange` 0 8)
        (:`0`
          (`AddComponent|NODE_AddChildActorComponent-218` :`RelativeTransform` _returnvalue))
        (:`1`
          (`AddComponent|NODE_AddChildActorComponent-219` :`RelativeTransform` _returnvalue))
        (:`2`
          (`AddComponent|NODE_AddChildActorComponent-220` :`RelativeTransform` _returnvalue))
        (:`3`
          (`AddComponent|NODE_AddChildActorComponent-221` :`RelativeTransform` _returnvalue))
        (:`4`
          (`AddComponent|NODE_AddChildActorComponent-222` :`RelativeTransform` _returnvalue))
        (:`5`
          (`AddComponent|NODE_AddChildActorComponent-223` :`RelativeTransform` _returnvalue))
        (:`6`
          (`AddComponent|NODE_AddChildActorComponent-224` :`RelativeTransform` _returnvalue))
        (:`7`
          (`AddComponent|NODE_AddChildActorComponent-225` :`RelativeTransform` _returnvalue))))
    (:`then_2`
      ; SP3
      (switch `int` (`KismetMathLibrary.RandomIntegerInRange` 0 8)
        (:`0`
          (`AddComponent|NODE_AddChildActorComponent-226` :`RelativeTransform` _returnvalue_6))
        (:`1`
          (`AddComponent|NODE_AddChildActorComponent-227` :`RelativeTransform` _returnvalue_6))
        (:`2`
          (`AddComponent|NODE_AddChildActorComponent-228` :`RelativeTransform` _returnvalue_6))
        (:`3`
          (`AddComponent|NODE_AddChildActorComponent-229` :`RelativeTransform` _returnvalue_6))
        (:`4`
          (`AddComponent|NODE_AddChildActorComponent-230` :`RelativeTransform` _returnvalue_6))
        (:`5`
          (`AddComponent|NODE_AddChildActorComponent-231` :`RelativeTransform` _returnvalue_6))
        (:`6`
          (`AddComponent|NODE_AddChildActorComponent-232` :`RelativeTransform` _returnvalue_6))
        (:`7`
          (`AddComponent|NODE_AddChildActorComponent-233` :`RelativeTransform` _returnvalue_6))))
    (:`then_3`
      ; SP4
      (switch `int` (`KismetMathLibrary.RandomIntegerInRange` 0 8)
        (:`0`
          (`AddComponent|NODE_AddChildActorComponent-234` :`RelativeTransform` _returnvalue_12))
        (:`1`
          (`AddComponent|NODE_AddChildActorComponent-235` :`RelativeTransform` _returnvalue_12))
        (:`2`
          (`AddComponent|NODE_AddChildActorComponent-236` :`RelativeTransform` _returnvalue_12))
        (:`3`
          (`AddComponent|NODE_AddChildActorComponent-237` :`RelativeTransform` _returnvalue_12))
        (:`4`
          (`AddComponent|NODE_AddChildActorComponent-238` :`RelativeTransform` _returnvalue_12))
        (:`5`
          (`AddComponent|NODE_AddChildActorComponent-239` :`RelativeTransform` _returnvalue_12))
        (:`6`
          (`AddComponent|NODE_AddChildActorComponent-240` :`RelativeTransform` _returnvalue_12))
        (:`7`
          (`AddComponent|NODE_AddChildActorComponent-241` :`RelativeTransform` _returnvalue_12))))
    (:`then_4`
      ; SP5
      (switch `int` (`KismetMathLibrary.RandomIntegerInRange` 0 8)
        (:`0`
          (`AddComponent|NODE_AddChildActorComponent-242` :`RelativeTransform` _returnvalue_24))
        (:`1`
          (`AddComponent|NODE_AddChildActorComponent-243` :`RelativeTransform` _returnvalue_24))
        (:`2`
          (`AddComponent|NODE_AddChildActorComponent-244` :`RelativeTransform` _returnvalue_24))
        (:`3`
          (`AddComponent|NODE_AddChildActorComponent-245` :`RelativeTransform` _returnvalue_24))
        (:`4`
          (`AddComponent|NODE_AddChildActorComponent-246` :`RelativeTransform` _returnvalue_24))
        (:`5`
          (`AddComponent|NODE_AddChildActorComponent-247` :`RelativeTransform` _returnvalue_24))
        (:`6`
          (`AddComponent|NODE_AddChildActorComponent-248` :`RelativeTransform` _returnvalue_24))
        (:`7`
          (`AddComponent|NODE_AddChildActorComponent-249` :`RelativeTransform` _returnvalue_24))))
    (:`then_5`
      ; SP6
      (switch `int` (`KismetMathLibrary.RandomIntegerInRange` 0 8)
        (:`0`
          (`AddComponent|NODE_AddChildActorComponent-250` :`RelativeTransform` _returnvalue_2))
        (:`1`
          (`AddComponent|NODE_AddChildActorComponent-251` :`RelativeTransform` _returnvalue_2))
        (:`2`
          (`AddComponent|NODE_AddChildActorComponent-252` :`RelativeTransform` _returnvalue_2))
        (:`3`
          (`AddComponent|NODE_AddChildActorComponent-253` :`RelativeTransform` _returnvalue_2))
        (:`4`
          (`AddComponent|NODE_AddChildActorComponent-254` :`RelativeTransform` _returnvalue_2))
        (:`5`
          (`AddComponent|NODE_AddChildActorComponent-255` :`RelativeTransform` _returnvalue_2))
        (:`6`
          (`AddComponent|NODE_AddChildActorComponent-256` :`RelativeTransform` _returnvalue_2))
        (:`7`
          (`AddComponent|NODE_AddChildActorComponent-257` :`RelativeTransform` _returnvalue_2))))
    (:`then_6`
      ; SP7
      (switch `int` (`KismetMathLibrary.RandomIntegerInRange` 0 8)
        (:`0`
          (`AddComponent|NODE_AddChildActorComponent-258` :`RelativeTransform` _returnvalue_3))
        (:`1`
          (`AddComponent|NODE_AddChildActorComponent-259` :`RelativeTransform` _returnvalue_3))
        (:`2`
          (`AddComponent|NODE_AddChildActorComponent-260` :`RelativeTransform` _returnvalue_3))
        (:`3`
          (`AddComponent|NODE_AddChildActorComponent-261` :`RelativeTransform` _returnvalue_3))
        (:`4`
          (`AddComponent|NODE_AddChildActorComponent-262` :`RelativeTransform` _returnvalue_3))
        (:`5`
          (`AddComponent|NODE_AddChildActorComponent-263` :`RelativeTransform` _returnvalue_3))
        (:`6`
          (`AddComponent|NODE_AddChildActorComponent-264` :`RelativeTransform` _returnvalue_3))
        (:`7`
          (`AddComponent|NODE_AddChildActorComponent-265` :`RelativeTransform` _returnvalue_3))))
    (:`then_7`
      ; SP8
      (switch `int` (`KismetMathLibrary.RandomIntegerInRange` 0 8)
        (:`0`
          (`AddComponent|NODE_AddChildActorComponent-266` :`RelativeTransform` _returnvalue_4))
        (:`1`
          (`AddComponent|NODE_AddChildActorComponent-267` :`RelativeTransform` _returnvalue_4))
        (:`2`
          (`AddComponent|NODE_AddChildActorComponent-268` :`RelativeTransform` _returnvalue_4))
        (:`3`
          (`AddComponent|NODE_AddChildActorComponent-269` :`RelativeTransform` _returnvalue_4))
        (:`4`
          (`AddComponent|NODE_AddChildActorComponent-270` :`RelativeTransform` _returnvalue_4))
        (:`5`
          (`AddComponent|NODE_AddChildActorComponent-271` :`RelativeTransform` _returnvalue_4))
        (:`6`
          (`AddComponent|NODE_AddChildActorComponent-272` :`RelativeTransform` _returnvalue_4))
        (:`7`
          (`AddComponent|NODE_AddChildActorComponent-273` :`RelativeTransform` _returnvalue_4))))
    (:`then_8`
      ; SP9
      (switch `int` (`KismetMathLibrary.RandomIntegerInRange` 0 8)
        (:`0`
          (`AddComponent|NODE_AddChildActorComponent-274` :`RelativeTransform` _returnvalue_5))
        (:`1`
          (`AddComponent|NODE_AddChildActorComponent-275` :`RelativeTransform` _returnvalue_5))
        (:`2`
          (`AddComponent|NODE_AddChildActorComponent-276` :`RelativeTransform` _returnvalue_5))
        (:`3`
          (`AddComponent|NODE_AddChildActorComponent-277` :`RelativeTransform` _returnvalue_5))
        (:`4`
          (`AddComponent|NODE_AddChildActorComponent-278` :`RelativeTransform` _returnvalue_5))
        (:`5`
          (`AddComponent|NODE_AddChildActorComponent-279` :`RelativeTransform` _returnvalue_5))
        (:`6`
          (`AddComponent|NODE_AddChildActorComponent-280` :`RelativeTransform` _returnvalue_5))
        (:`7`
          (`AddComponent|NODE_AddChildActorComponent-281` :`RelativeTransform` _returnvalue_5))))
    (:`then_9`
      ; SP10
      (switch `int` (`KismetMathLibrary.RandomIntegerInRange` 0 8)
        (:`0`
          (`AddComponent|NODE_AddChildActorComponent-282` :`RelativeTransform` _returnvalue_7))
        (:`1`
          (`AddComponent|NODE_AddChildActorComponent-283` :`RelativeTransform` _returnvalue_7))
        (:`2`
          (`AddComponent|NODE_AddChildActorComponent-284` :`RelativeTransform` _returnvalue_7))
        (:`3`
          (`AddComponent|NODE_AddChildActorComponent-285` :`RelativeTransform` _returnvalue_7))
        (:`4`
          (`AddComponent|NODE_AddChildActorComponent-286` :`RelativeTransform` _returnvalue_7))
        (:`5`
          (`AddComponent|NODE_AddChildActorComponent-287` :`RelativeTransform` _returnvalue_7))
        (:`6`
          (`AddComponent|NODE_AddChildActorComponent-288` :`RelativeTransform` _returnvalue_7))
        (:`7`
          (`AddComponent|NODE_AddChildActorComponent-289` :`RelativeTransform` _returnvalue_7))))
    (:`then_10`
      ; SP11
      (switch `int` (`KismetMathLibrary.RandomIntegerInRange` 0 8)
        (:`0`
          (`AddComponent|NODE_AddChildActorComponent-290` :`RelativeTransform` _returnvalue_8))
        (:`1`
          (`AddComponent|NODE_AddChildActorComponent-291` :`RelativeTransform` _returnvalue_8))
        (:`2`
          (`AddComponent|NODE_AddChildActorComponent-292` :`RelativeTransform` _returnvalue_8))
        (:`3`
          (`AddComponent|NODE_AddChildActorComponent-293` :`RelativeTransform` _returnvalue_8))
        (:`4`
          (`AddComponent|NODE_AddChildActorComponent-294` :`RelativeTransform` _returnvalue_8))
        (:`5`
          (`AddComponent|NODE_AddChildActorComponent-295` :`RelativeTransform` _returnvalue_8))
        (:`6`
          (`AddComponent|NODE_AddChildActorComponent-296` :`RelativeTransform` _returnvalue_8))
        (:`7`
          (`AddComponent|NODE_AddChildActorComponent-297` :`RelativeTransform` _returnvalue_8))))
    (:`then_11`
      ; SP12
      (switch `int` (`KismetMathLibrary.RandomIntegerInRange` 0 8)
        (:`0`
          (`AddComponent|NODE_AddChildActorComponent-298` :`RelativeTransform` _returnvalue_9))
        (:`1`
          (`AddComponent|NODE_AddChildActorComponent-299` :`RelativeTransform` _returnvalue_9))
        (:`2`
          (`AddComponent|NODE_AddChildActorComponent-300` :`RelativeTransform` _returnvalue_9))
        (:`3`
          (`AddComponent|NODE_AddChildActorComponent-301` :`RelativeTransform` _returnvalue_9))
        (:`4`
          (`AddComponent|NODE_AddChildActorComponent-302` :`RelativeTransform` _returnvalue_9))
        (:`5`
          (`AddComponent|NODE_AddChildActorComponent-303` :`RelativeTransform` _returnvalue_9))
        (:`6`
          (`AddComponent|NODE_AddChildActorComponent-304` :`RelativeTransform` _returnvalue_9))
        (:`7`
          (`AddComponent|NODE_AddChildActorComponent-305` :`RelativeTransform` _returnvalue_9))))
    (:`then_12`
      ; SP13
      (switch `int` (`KismetMathLibrary.RandomIntegerInRange` 0 8)
        (:`0`
          (`AddComponent|NODE_AddChildActorComponent-306` :`RelativeTransform` _returnvalue_13))
        (:`1`
          (`AddComponent|NODE_AddChildActorComponent-307` :`RelativeTransform` _returnvalue_13))
        (:`2`
          (`AddComponent|NODE_AddChildActorComponent-308` :`RelativeTransform` _returnvalue_13))
        (:`3`
          (`AddComponent|NODE_AddChildActorComponent-309` :`RelativeTransform` _returnvalue_13))
        (:`4`
          (`AddComponent|NODE_AddChildActorComponent-310` :`RelativeTransform` _returnvalue_13))
        (:`5`
          (`AddComponent|NODE_AddChildActorComponent-311` :`RelativeTransform` _returnvalue_13))
        (:`6`
          (`AddComponent|NODE_AddChildActorComponent-312` :`RelativeTransform` _returnvalue_13))
        (:`7`
          (`AddComponent|NODE_AddChildActorComponent-313` :`RelativeTransform` _returnvalue_13))))
    (:`then_13`
      ; SP14
      (switch `int` (`KismetMathLibrary.RandomIntegerInRange` 0 8)
        (:`0`
          (`AddComponent|NODE_AddChildActorComponent-314` :`RelativeTransform` _returnvalue_14))
        (:`1`
          (`AddComponent|NODE_AddChildActorComponent-315` :`RelativeTransform` _returnvalue_14))
        (:`2`
          (`AddComponent|NODE_AddChildActorComponent-316` :`RelativeTransform` _returnvalue_14))
        (:`3`
          (`AddComponent|NODE_AddChildActorComponent-317` :`RelativeTransform` _returnvalue_14))
        (:`4`
          (`AddComponent|NODE_AddChildActorComponent-318` :`RelativeTransform` _returnvalue_14))
        (:`5`
          (`AddComponent|NODE_AddChildActorComponent-319` :`RelativeTransform` _returnvalue_14))
        (:`6`
          (`AddComponent|NODE_AddChildActorComponent-320` :`RelativeTransform` _returnvalue_14))
        (:`7`
          (`AddComponent|NODE_AddChildActorComponent-321` :`RelativeTransform` _returnvalue_14))))
    (:`then_14`
      ; SP15
      (switch `int` (`KismetMathLibrary.RandomIntegerInRange` 0 8)
        (:`0`
          (`AddComponent|NODE_AddChildActorComponent-322` :`RelativeTransform` _returnvalue_15))
        (:`1`
          (`AddComponent|NODE_AddChildActorComponent-323` :`RelativeTransform` _returnvalue_15))
        (:`2`
          (`AddComponent|NODE_AddChildActorComponent-324` :`RelativeTransform` _returnvalue_15))
        (:`3`
          (`AddComponent|NODE_AddChildActorComponent-325` :`RelativeTransform` _returnvalue_15))
        (:`4`
          (`AddComponent|NODE_AddChildActorComponent-326` :`RelativeTransform` _returnvalue_15))
        (:`5`
          (`AddComponent|NODE_AddChildActorComponent-327` :`RelativeTransform` _returnvalue_15))
        (:`6`
          (`AddComponent|NODE_AddChildActorComponent-328` :`RelativeTransform` _returnvalue_15))
        (:`7`
          (`AddComponent|NODE_AddChildActorComponent-329` :`RelativeTransform` _returnvalue_15))))
    (:`then_15`
      ; SP16
      (switch `int` (`KismetMathLibrary.RandomIntegerInRange` 0 8)
        (:`0`
          (`AddComponent|NODE_AddChildActorComponent-330` :`RelativeTransform` _returnvalue_16))
        (:`1`
          (`AddComponent|NODE_AddChildActorComponent-331` :`RelativeTransform` _returnvalue_16))
        (:`2`
          (`AddComponent|NODE_AddChildActorComponent-332` :`RelativeTransform` _returnvalue_16))
        (:`3`
          (`AddComponent|NODE_AddChildActorComponent-333` :`RelativeTransform` _returnvalue_16))
        (:`4`
          (`AddComponent|NODE_AddChildActorComponent-334` :`RelativeTransform` _returnvalue_16))
        (:`5`
          (`AddComponent|NODE_AddChildActorComponent-335` :`RelativeTransform` _returnvalue_16))
        (:`6`
          (`AddComponent|NODE_AddChildActorComponent-336` :`RelativeTransform` _returnvalue_16))
        (:`7`
          (`AddComponent|NODE_AddChildActorComponent-337` :`RelativeTransform` _returnvalue_16))))
    (:`then_16`
      ; SP17
      (switch `int` (`KismetMathLibrary.RandomIntegerInRange` 0 8)
        (:`0`
          (`AddComponent|NODE_AddChildActorComponent-338` :`RelativeTransform` _returnvalue_17))
        (:`1`
          (`AddComponent|NODE_AddChildActorComponent-339` :`RelativeTransform` _returnvalue_17))
        (:`2`
          (`AddComponent|NODE_AddChildActorComponent-340` :`RelativeTransform` _returnvalue_17))
        (:`3`
          (`AddComponent|NODE_AddChildActorComponent-341` :`RelativeTransform` _returnvalue_17))
        (:`4`
          (`AddComponent|NODE_AddChildActorComponent-342` :`RelativeTransform` _returnvalue_17))
        (:`5`
          (`AddComponent|NODE_AddChildActorComponent-343` :`RelativeTransform` _returnvalue_17))
        (:`6`
          (`AddComponent|NODE_AddChildActorComponent-344` :`RelativeTransform` _returnvalue_17))
        (:`7`
          (`AddComponent|NODE_AddChildActorComponent-345` :`RelativeTransform` _returnvalue_17))))
    (:`then_17`
      ; SP18
      (switch `int` (`KismetMathLibrary.RandomIntegerInRange` 0 8)
        (:`0`
          (`AddComponent|NODE_AddChildActorComponent-346` :`RelativeTransform` _returnvalue_18))
        (:`1`
          (`AddComponent|NODE_AddChildActorComponent-347` :`RelativeTransform` _returnvalue_18))
        (:`2`
          (`AddComponent|NODE_AddChildActorComponent-348` :`RelativeTransform` _returnvalue_18))
        (:`3`
          (`AddComponent|NODE_AddChildActorComponent-349` :`RelativeTransform` _returnvalue_18))
        (:`4`
          (`AddComponent|NODE_AddChildActorComponent-350` :`RelativeTransform` _returnvalue_18))
        (:`5`
          (`AddComponent|NODE_AddChildActorComponent-351` :`RelativeTransform` _returnvalue_18))
        (:`6`
          (`AddComponent|NODE_AddChildActorComponent-352` :`RelativeTransform` _returnvalue_18))
        (:`7`
          (`AddComponent|NODE_AddChildActorComponent-353` :`RelativeTransform` _returnvalue_18))))
    (:`then_18`
      ; SP19
      (switch `int` (`KismetMathLibrary.RandomIntegerInRange` 0 8)
        (:`0`
          (`AddComponent|NODE_AddChildActorComponent-354` :`RelativeTransform` _returnvalue_19))
        (:`1`
          (`AddComponent|NODE_AddChildActorComponent-355` :`RelativeTransform` _returnvalue_19))
        (:`2`
          (`AddComponent|NODE_AddChildActorComponent-356` :`RelativeTransform` _returnvalue_19))
        (:`3`
          (`AddComponent|NODE_AddChildActorComponent-357` :`RelativeTransform` _returnvalue_19))
        (:`4`
          (`AddComponent|NODE_AddChildActorComponent-358` :`RelativeTransform` _returnvalue_19))
        (:`5`
          (`AddComponent|NODE_AddChildActorComponent-359` :`RelativeTransform` _returnvalue_19))
        (:`6`
          (`AddComponent|NODE_AddChildActorComponent-360` :`RelativeTransform` _returnvalue_19))
        (:`7`
          (`AddComponent|NODE_AddChildActorComponent-361` :`RelativeTransform` _returnvalue_19))))
    (:`then_19`
      ; SP20
      (switch `int` (`KismetMathLibrary.RandomIntegerInRange` 0 8)
        (:`0`
          (`AddComponent|NODE_AddChildActorComponent-362` :`RelativeTransform` _returnvalue_20))
        (:`1`
          (`AddComponent|NODE_AddChildActorComponent-363` :`RelativeTransform` _returnvalue_20))
        (:`2`
          (`AddComponent|NODE_AddChildActorComponent-364` :`RelativeTransform` _returnvalue_20))
        (:`3`
          (`AddComponent|NODE_AddChildActorComponent-365` :`RelativeTransform` _returnvalue_20))
        (:`4`
          (`AddComponent|NODE_AddChildActorComponent-366` :`RelativeTransform` _returnvalue_20))
        (:`5`
          (`AddComponent|NODE_AddChildActorComponent-367` :`RelativeTransform` _returnvalue_20))
        (:`6`
          (`AddComponent|NODE_AddChildActorComponent-368` :`RelativeTransform` _returnvalue_20))
        (:`7`
          (`AddComponent|NODE_AddChildActorComponent-369` :`RelativeTransform` _returnvalue_20))))
    (:`then_20`
      ; SP21
      (switch `int` (`KismetMathLibrary.RandomIntegerInRange` 0 8)
        (:`0`
          (`AddComponent|NODE_AddChildActorComponent-370` :`RelativeTransform` _returnvalue_21))
        (:`1`
          (`AddComponent|NODE_AddChildActorComponent-371` :`RelativeTransform` _returnvalue_21))
        (:`2`
          (`AddComponent|NODE_AddChildActorComponent-372` :`RelativeTransform` _returnvalue_21))
        (:`3`
          (`AddComponent|NODE_AddChildActorComponent-373` :`RelativeTransform` _returnvalue_21))
        (:`4`
          (`AddComponent|NODE_AddChildActorComponent-374` :`RelativeTransform` _returnvalue_21))
        (:`5`
          (`AddComponent|NODE_AddChildActorComponent-375` :`RelativeTransform` _returnvalue_21))
        (:`6`
          (`AddComponent|NODE_AddChildActorComponent-376` :`RelativeTransform` _returnvalue_21))
        (:`7`
          (`AddComponent|NODE_AddChildActorComponent-377` :`RelativeTransform` _returnvalue_21))))
    (:`then_21`
      ; SP22
      (switch `int` (`KismetMathLibrary.RandomIntegerInRange` 0 8)
        (:`0`
          (`AddComponent|NODE_AddChildActorComponent-378` :`RelativeTransform` _returnvalue_22))
        (:`1`
          (`AddComponent|NODE_AddChildActorComponent-379` :`RelativeTransform` _returnvalue_22))
        (:`2`
          (`AddComponent|NODE_AddChildActorComponent-380` :`RelativeTransform` _returnvalue_22))
        (:`3`
          (`AddComponent|NODE_AddChildActorComponent-381` :`RelativeTransform` _returnvalue_22))
        (:`4`
          (`AddComponent|NODE_AddChildActorComponent-382` :`RelativeTransform` _returnvalue_22))
        (:`5`
          (`AddComponent|NODE_AddChildActorComponent-383` :`RelativeTransform` _returnvalue_22))
        (:`6`
          (`AddComponent|NODE_AddChildActorComponent-384` :`RelativeTransform` _returnvalue_22))
        (:`7`
          (`AddComponent|NODE_AddChildActorComponent-385` :`RelativeTransform` _returnvalue_22))))
    (:`then_22`
      ; SP23
      (switch `int` (`KismetMathLibrary.RandomIntegerInRange` 0 8)
        (:`0`
          (`AddComponent|NODE_AddChildActorComponent-386` :`RelativeTransform` _returnvalue_23))
        (:`1`
          (`AddComponent|NODE_AddChildActorComponent-387` :`RelativeTransform` _returnvalue_23))
        (:`2`
          (`AddComponent|NODE_AddChildActorComponent-388` :`RelativeTransform` _returnvalue_23))
        (:`3`
          (`AddComponent|NODE_AddChildActorComponent-389` :`RelativeTransform` _returnvalue_23))
        (:`4`
          (`AddComponent|NODE_AddChildActorComponent-390` :`RelativeTransform` _returnvalue_23))
        (:`5`
          (`AddComponent|NODE_AddChildActorComponent-391` :`RelativeTransform` _returnvalue_23))
        (:`6`
          (`AddComponent|NODE_AddChildActorComponent-392` :`RelativeTransform` _returnvalue_23))
        (:`7`
          (`AddComponent|NODE_AddChildActorComponent-393` :`RelativeTransform` _returnvalue_23))))
    (:`then_24`
      ; SP25
      (switch `int` (`KismetMathLibrary.RandomIntegerInRange` 0 8)
        (:`0`
          (`AddComponent|NODE_AddChildActorComponent-410` :`RelativeTransform` _returnvalue_10))
        (:`1`
          (`AddComponent|NODE_AddChildActorComponent-411` :`RelativeTransform` _returnvalue_10))
        (:`2`
          (`AddComponent|NODE_AddChildActorComponent-412` :`RelativeTransform` _returnvalue_10))
        (:`3`
          (`AddComponent|NODE_AddChildActorComponent-413` :`RelativeTransform` _returnvalue_10))
        (:`4`
          (`AddComponent|NODE_AddChildActorComponent-414` :`RelativeTransform` _returnvalue_10))
        (:`5`
          (`AddComponent|NODE_AddChildActorComponent-415` :`RelativeTransform` _returnvalue_10))
        (:`6`
          (`AddComponent|NODE_AddChildActorComponent-416` :`RelativeTransform` _returnvalue_10))
        (:`7`
          (`AddComponent|NODE_AddChildActorComponent-417` :`RelativeTransform` _returnvalue_10))))))

(fn `UserConstructionScript`
  (`self.Spawn rocks`))