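; Magnet power-up for the runner game that temporarily activates the player character's magnet state on overlap.
; Pickup plays a sound and, if no magnet is active, sets the character flag and game mode's MagnetTimer.
; A delayed loop counts that timer down while a parallel Delay clears the flag and destroys the actor.
; Overlapping an obstacle wall destroys the pickup.
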(event `self.ReceiveActorBeginOverlap`
  (params (OtherActor :type "Actor Object Reference"))
  (`|ExecutionSequence`
    (:`then_0`
      (bind _asbp_runner_character (cast `/Game/Runner/Blueprints/BP_RunnerCharacter` OtherActor))
      (bind _asbp_runner_game_mode (cast `/Game/Runner/Blueprints/BP_RunnerGameMode` (`GameplayStatics.GetGameMode`)))
      (`GameplayStatics.PlaySound2D` "/Game/Runner/Audio/Effects/PowerUp.PowerUp" 1.0 1.0 0.0 null null)
      (`self.SetActorHiddenInGame` false)
      (if (not (`/Game/Runner/Blueprints/BP_RunnerCharacter.Is Magnet Active?` _asbp_runner_character))
        (set `/Game/Runner/Blueprints/BP_RunnerCharacter.Is Magnet Active?` true _asbp_runner_character)
        (set `/Game/Runner/Blueprints/BP_RunnerGameMode.Magnet Timer` 6.0 _asbp_runner_game_mode)
        (`KismetSystemLibrary.PrintString` "MagnetActive")
        (`|ExecutionSequence`
          (:`then_0`
            (`/Game/Runner/Blueprints/Input/ForLoopWDelay.ForLoopWithDelay` 0 5 1.0
              (:`Loop Body`
                (bind _result (`/Engine/EditorBlueprintResources/StandardMacros.DecrementFloat` (`/Game/Runner/Blueprints/BP_RunnerGameMode.Magnet Timer` _asbp_runner_game_mode))
                  (:`  `
                    (bind _output_get (set `/Game/Runner/Blueprints/BP_RunnerGameMode.Magnet Timer` (`KismetMathLibrary.FMax` _result) _asbp_runner_game_mode))
                    (`KismetSystemLibrary.PrintString` (`KismetStringLibrary.Conv_DoubleToString` _output_get) true true (struct :`R` 0.123732 :`G` 1.0 :`B` 0.191396 :`A` 1.0)))))))
          (:`then_1`
            (`KismetSystemLibrary.Delay` 5.2)
            (bind _asbp_runner_character_2 (cast `/Game/Runner/Blueprints/BP_RunnerCharacter` (`GameplayStatics.GetPlayerCharacter` 0)))
            (set `/Game/Runner/Blueprints/BP_RunnerCharacter.Is Magnet Active?` false _asbp_runner_character_2)
            (`KismetSystemLibrary.PrintString` "Magnet Not Active")
            (`self.K2_DestroyActor`)))))
    (:`then_1`
      (cast `/Game/Runner/Blueprints/Obstacles/BP_Obstacles_Wall` OtherActor)
      (`self.K2_DestroyActor`))))

(fn `UserConstructionScript`)