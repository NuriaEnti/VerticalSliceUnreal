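; BP_Misil is a missile obstacle for a runner game that launches when the runner character enters its trigger.
; OverlapCollision starts a flight sound and a Timeline that lerps the mesh's current world X toward the Arrow's, then destroys the actor after a delay.
; MisilCollision plays an explosion and calls the runner's Death(), destroying the missile on true or pausing the game after a delay on false.
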(event `self.MisilCollision.OnComponentBeginOverlap`
  (params (OverlappedComponent :type "PrimitiveComponent Object Reference") (OtherActor :type "Actor Object Reference") (OtherComp :type "PrimitiveComponent Object Reference") (OtherBodyIndex :type Integer) (bFromSweep :type Boolean) (SweepResult :type "HitResult Structure (by ref)"))
  (bind _asbp_runner_character (cast `/Game/Runner/Blueprints/BP_RunnerCharacter` OtherActor))
  (`GameplayStatics.PlaySound2D` "/Game/Runner/Audio/Effects/Explosion.Explosion" 1.0 1.0 0.0 null null)
  (bind _wasshielded (`/Game/Runner/Blueprints/BP_RunnerCharacter.Death` _asbp_runner_character))
  (if _wasshielded
    (`self.K2_DestroyActor`)
    (else
      (`KismetSystemLibrary.Delay` 1.0)
      (`GameplayStatics.SetGamePaused` true))))

(event `self.Overlap Collision.OnComponentBeginOverlap`
  (params (OverlappedComponent :type "PrimitiveComponent Object Reference") (OtherActor :type "Actor Object Reference") (OtherComp :type "PrimitiveComponent Object Reference") (OtherBodyIndex :type Integer) (bFromSweep :type Boolean) (SweepResult :type "HitResult Structure (by ref)"))
  (bind _staticmesh (`self.StaticMesh`))
  (cast `/Game/Runner/Blueprints/BP_RunnerCharacter` OtherActor)
  (`GameplayStatics.SpawnSoundAttached` "/Game/Runner/Audio/Effects/RocketFly.RocketFly" (`self.StaticMesh`) "None" (0.0 0.0 0.0) (struct) "KeepRelativeOffset" false 1.0 1.0 0.0 null null)
  (bind (_direction _move_obstacle) (`Timeline|Timeline`)
    (:`Update`
      (`SceneComponent.K2_SetWorldLocation` _staticmesh (`KismetMathLibrary.MakeVector` (`KismetMathLibrary.Lerp` (.x (`SceneComponent.K2_GetComponentLocation` _staticmesh)) (.x (`SceneComponent.K2_GetComponentLocation` (`self.Arrow`))) _move_obstacle) (.y (`SceneComponent.K2_GetComponentLocation` _staticmesh)) (.z (`SceneComponent.K2_GetComponentLocation` _staticmesh))) false false))
    (:`Finished`
      (`KismetSystemLibrary.Delay` 5.0)
      (`self.K2_DestroyActor`))))

(fn `UserConstructionScript`
  (`parent.UserConstructionScript`))