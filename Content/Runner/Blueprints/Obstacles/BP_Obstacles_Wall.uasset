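; BP_Obstacles_Wall is a wall obstacle for the runner game that triggers the runner character's death on overlap.
; When a BP_RunnerCharacter overlaps it, the wall calls that character's Death function and branches on the returned value.
; A true result destroys the wall, while a false result pauses the game after a short delay.
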(event `self.ReceiveActorBeginOverlap`
  (params (OtherActor :type "Actor Object Reference"))
  (bind _asbp_runner_character (cast `/Game/Runner/Blueprints/BP_RunnerCharacter` OtherActor))
  (bind _wasshielded (`/Game/Runner/Blueprints/BP_RunnerCharacter.Death` _asbp_runner_character))
  (if _wasshielded
    (`self.K2_DestroyActor`)
    (else
      (`KismetSystemLibrary.Delay` 1.0)
      (`GameplayStatics.SetGamePaused` true))))

(fn `UserConstructionScript`
  (`parent.UserConstructionScript`))