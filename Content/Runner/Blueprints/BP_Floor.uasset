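; Floor tile for a lane-based runner that populates itself with random obstacles, coins and power-ups.
; The construction script generates per-lane arrow spawn points, shuffles them and adds child actors, with Game Mode floor counters limiting power-ups and moving obstacles.
; Box overlap tells the Game Mode to extend the floor, raises player speed within a clamp and adds points.
; GetAttachPoint exposes the Arrow's world transform.
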(event `self.Box.OnComponentBeginOverlap`
  (params (OverlappedComponent :type "PrimitiveComponent Object Reference") (OtherActor :type "Actor Object Reference") (OtherComp :type "PrimitiveComponent Object Reference") (OtherBodyIndex :type Integer) (bFromSweep :type Boolean) (SweepResult :type "HitResult Structure (by ref)"))
  ; Extend Floor
  (bind _asbp_runner_game_mode (cast `/Game/Runner/Blueprints/BP_RunnerGameMode` (`GameplayStatics.GetGameMode`)))
  (`/Game/Runner/Blueprints/BP_RunnerGameMode.Extend Floor` _asbp_runner_game_mode)
  ; Change Speed
  (bind _asbp_runner_character (cast `/Game/Runner/Blueprints/BP_RunnerCharacter` (`GameplayStatics.GetPlayerCharacter` 0)))
  (bind _charactermovement (`Character.CharacterMovement` _asbp_runner_character))
  (bind _output_get (set `CharacterMovementComponent.MaxWalkSpeed` (`KismetMathLibrary.FClamp` (* (`CharacterMovementComponent.MaxWalkSpeed` _charactermovement) 1.01) 700.0 2000.0) _charactermovement))
  (`KismetSystemLibrary.PrintString` (`KismetStringLibrary.Conv_DoubleToString` _output_get))
  ; set current score
  (bind _asbp_runner_game_mode_2 (cast `/Game/Runner/Blueprints/BP_RunnerGameMode` (`GameplayStatics.GetGameMode`)))
  (set `/Game/Runner/Blueprints/BP_RunnerGameMode.Current Points` (+ (* (`/Game/Runner/Blueprints/BP_RunnerGameMode.Points Multi` _asbp_runner_game_mode_2) 1) (`/Game/Runner/Blueprints/BP_RunnerGameMode.Current Points` _asbp_runner_game_mode_2)) _asbp_runner_game_mode_2))

(fn `Coin Spawn Points`
  (for _array_element (`self.Lane Position`)
    (for _index (range 10)
      (bind _returnvalue (`AddComponent|NODE_AddArrowComponent-1` :`RelativeTransform` (`KismetMathLibrary.MakeTransform` (`KismetMathLibrary.MakeVector` (* _index 75.0) _array_element))))
      (`ArrowComponent.SetArrowColor` _returnvalue (struct :`R` 1.0 :`G` 1.0 :`B` 1.0 :`A` 1.0))
      (`KismetArrayLibrary.Array_Add` (`self.CSpawnPoints`) (`SceneComponent.K2_GetComponentToWorld` _returnvalue)))))

(fn `Get AttachPoint`
  (returns (ReturnValue :type "Transform Structure"))
  (return (`SceneComponent.K2_GetComponentToWorld` (`self.Arrow`))))

(fn `Powerup Spawn Points`
  (for _array_element (`self.Lane Position`)
    (for _index (range 1 3)
      (bind _returnvalue (`AddComponent|NODE_AddArrowComponent-2` :`RelativeTransform` (`KismetMathLibrary.MakeTransform` (`KismetMathLibrary.MakeVector` (* _index 250.0) _array_element))))
      (`ArrowComponent.SetArrowColor` _returnvalue (struct :`R` 0.921405 :`B` 1.0 :`A` 1.0))
      (`KismetArrayLibrary.Array_Add` (`self.PSpawn Points`) (`SceneComponent.K2_GetComponentToWorld` _returnvalue)))))

(fn `Setup Spawn Points`
  (bind _relativelocation_x (`KismetMathLibrary.BreakVector` (`SceneComponent.RelativeLocation` (`self.Arrow`))))
  (for _array_element (`self.Lane Position`)
    (for _index (range 2)
      (bind _returnvalue (`AddComponent|NODE_AddArrowComponent-0` :`RelativeTransform` (`KismetMathLibrary.MakeTransform` (`KismetMathLibrary.MakeVector` (* _index _relativelocation_x) _array_element))))
      (`KismetArrayLibrary.Array_Add` (`self.Spawn Points`) (`SceneComponent.K2_GetComponentToWorld` _returnvalue)))))

(fn `Spawn Coins`
  (locals (`Random Spawn Points` :type "Array of Transform Structure"))
  (bind _output_get (set `local.Random Spawn Points` (`self.CSpawnPoints`)))
  (`KismetArrayLibrary.Array_Shuffle` _output_get)
  (for _index (range (+ (`KismetMathLibrary.RandomIntegerInRange` 0 2) 1))
    (switch `int` 0
      (:`0`
        (`AddComponent|NODE_AddChildActorComponent-12` :`RelativeTransform` (`KismetMathLibrary.MakeRelativeTransform` (`|GetArrayItem` (`local.Random Spawn Points`) _index) (`self.GetTransform`)))))))

(fn `Spawn Moving Obstacles`
  (params (Selection :type Integer) (RelativeTransform :type "Transform Structure"))
  (bind _asbp_runner_game_mode (cast `/Game/Runner/Blueprints/BP_RunnerGameMode` (`GameplayStatics.GetGameMode`)))
  (if (> (`/Game/Runner/Blueprints/BP_RunnerGameMode.Floor Count For Obstacles` _asbp_runner_game_mode) (`KismetMathLibrary.RandomIntegerInRange` 10 20))
    (switch `int` Selection
      (:`0`
        (`AddComponent|NODE_AddChildActorComponent-15` :`RelativeTransform` RelativeTransform)
        (set `/Game/Runner/Blueprints/BP_RunnerGameMode.Floor Count For Obstacles` 0 _asbp_runner_game_mode)))))

(fn `Spawn Obstacles`
  (locals (`Random Spawn Points` :type "Array of Transform Structure"))
  (bind _output_get (set `local.Random Spawn Points` (`self.Spawn Points`)))
  (`KismetArrayLibrary.Array_Shuffle` _output_get)
  (for _index (range (+ (`KismetMathLibrary.RandomIntegerInRange` 0 1) 1))
    (switch `int` (`KismetMathLibrary.RandomIntegerInRange` 0 2)
      (:`0`
        (bind _returnvalue (`KismetMathLibrary.MakeRelativeTransform` (`|GetArrayItem` (`local.Random Spawn Points`) _index) (`self.GetTransform`)))
        (`AddComponent|NODE_AddChildActorComponent-0` :`RelativeTransform` _returnvalue))
      (:`1`
        (`AddComponent|NODE_AddChildActorComponent-1` :`RelativeTransform` _returnvalue))
      (:`2`
        (`self.Spawn Moving Obstacles` 0 _returnvalue)))))

(fn `Spawn PowerUps`
  (locals (`Random Spawn Points` :type "Array of Transform Structure"))
  (bind _returnvalue (`KismetMathLibrary.MakeRelativeTransform` (`|GetArrayItem` (`local.Random Spawn Points`)) (`self.GetTransform`)))
  (bind _asbp_runner_game_mode (cast `/Game/Runner/Blueprints/BP_RunnerGameMode` (`GameplayStatics.GetGameMode`)))
  (if (> (`/Game/Runner/Blueprints/BP_RunnerGameMode.Floor Count` _asbp_runner_game_mode) 10)
    (bind _output_get (set `local.Random Spawn Points` (`self.PSpawn Points`)))
    (`KismetArrayLibrary.Array_Shuffle` _output_get)
    (switch `int` (`KismetMathLibrary.RandomIntegerInRange` 0 1)
      (:`0`
        (`AddComponent|NODE_AddChildActorComponent-13` :`RelativeTransform` _returnvalue))
      (:`1`
        (`AddComponent|NODE_AddChildActorComponent-16` :`RelativeTransform` _returnvalue)))
    (set `/Game/Runner/Blueprints/BP_RunnerGameMode.Floor Count` 0 _asbp_runner_game_mode)))

(fn `UserConstructionScript`
  (`self.Setup Spawn Points`)
  (`self.Spawn Obstacles`)
  (`self.Coin Spawn Points`)
  (`self.Spawn Coins`)
  (`self.Powerup Spawn Points`)
  (`self.Spawn PowerUps`))