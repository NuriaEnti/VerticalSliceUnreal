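; Game mode for an endless runner that builds the track and scenery, times power-ups and loads saved coins.
; Floor and environment actors chain from the previous piece's attach point, with older ones destroyed as the track extends.
; An environment countdown spawns a one-time portal at the floor's end, and ChangeEnviro swaps in the second environment set.
; Looping timers run magnet and multi-coin countdowns, broadcast progress and clear player flags on expiry.
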(event Custom|ExtendEnvironm
  (bind _bp_enviroment (Variables|Default|GetBP_Enviroment))
  (bind _bp_otherenviroment (Variables|Default|GetBP_OtherEnviroment))
  (bind _output (Utilities|Array|Get(acopy) _bp_enviroment))
  (bind _output_2 (Utilities|Array|Get(acopy) _bp_otherenviroment))
  (CallFunction|AddEnviroment)
  (Utilities|FlowControl|Sequence
    (:then_0
      (if (> (Utilities|Array|Length (Variables|Default|GetBP_Enviroment)) 0)
        (Utilities|FlowControl|Delay 0.75)
        (Actor|DestroyActor _output)
        (Utilities|Array|RemoveItem _bp_enviroment _output)))
    (:then_1
      (if (Variables|Default|GetUseOtherEnviro)
        (if (> (Utilities|Array|Length (Variables|Default|GetBP_OtherEnviroment)) 2)
          (Utilities|FlowControl|Delay 0.75)
          (Actor|DestroyActor _output_2)
          (Utilities|Array|RemoveItem _bp_otherenviroment _output_2))))))

(event Custom|EnableMagnetPowerUp
  (Development|PrintString "MagnetActive")
  (if (Utilities|Time|IsValidTimerHandle (Variables|PowerUps|GetMagentTimerHdl))
    (Utilities|Time|ClearandInvalidateTimerbyHandle (Variables|PowerUps|GetMagentTimerHdl)))
  (Variables|PowerUps|SetMagnet%20Timer 6.0)
  (bind _returnvalue (Utilities|Time|SetTimerbyEvent (delegate Custom|UpdateMagentTimer) 0.002 true true))
  (Variables|PowerUps|SetMagentTimerHdl _returnvalue))

(event Custom|UpdateMagentTimer
  (bind _output_get (Variables|PowerUps|SetMagnet%20Timer (- (Variables|PowerUps|GetMagnet%20Timer) (Utilities|Time|GetWorldDeltaSeconds))))
  (Default|CallOnMagnetTimerUpdated _output_get 6.0 (|(MagnetTimer<=0.010000) _output_get))
  (if (|(MagnetTimer<=0.010000) _output_get)
    (Utilities|Time|ClearandInvalidateTimerbyHandle (Variables|PowerUps|GetMagentTimerHdl))
    (Variables|/Game/Runner/Blueprints/BP_RunnerCharacter.BP_RunnerCharacter_C|SetIs%20Magnet%20Active? (Variables|Default|GetPlayerRef) false)
    (Development|PrintString "MagnetDisabled")))

(event Custom|EnableMultiCoinsPowUp
  (if (Utilities|Time|IsValidTimerHandle (Variables|PowerUps|GetCoinsTimerHdl))
    (Utilities|Time|ClearandInvalidateTimerbyHandle (Variables|PowerUps|GetCoinsTimerHdl)))
  (Variables|PowerUps|SetMultiCoinsTimer 1e+01)
  (bind _returnvalue (Utilities|Time|SetTimerbyEvent (delegate Custom|UpdateCoinsPowUp) 0.002 true true))
  (Variables|PowerUps|SetCoinsTimerHdl _returnvalue))

(event Custom|UpdateCoinsPowUp
  (bind _returnvalue (|({50CB3D8C-48F4-7985-D054-5FAA2BDC7F61}<=0.010000)))
  (bind _output_get (Variables|PowerUps|SetMultiCoinsTimer (|({50CB3D8C-48F4-7985-D054-5FAA2BDC7F61}-dt) (Utilities|Time|GetWorldDeltaSeconds))))
  (Default|CallOnMultiCoinsTimerUpdt _output_get 1e+01 _returnvalue)
  (if _returnvalue
    (Utilities|Time|ClearandInvalidateTimerbyHandle (Variables|PowerUps|GetCoinsTimerHdl))
    (Variables|/Game/Runner/Blueprints/BP_RunnerCharacter.BP_RunnerCharacter_C|SetIsCoinsPowUpActive (Variables|Default|GetPlayerRef) false)))

(event EventBeginPlay
  (Utilities|FlowControl|Sequence
    (:then_0
      (for _index (range 0 (- (Variables|Default|GetNumberOfTiles) 1))
        (CallFunction|AddFloor)))
    (:then_1
      (for _index_2 (range 0 5)
        (CallFunction|AddEnviroment)))
    (:then_2
      (bind _asbp_runner_character (Utilities|Casting|CastToBP_RunnerCharacter (Game|GetPlayerCharacter 0)))
      (bind _output_get (Variables|Default|SetPlayerRef _asbp_runner_character))
      (Default|UpdateCoins _output_get)
      (bind _returnvalue (SaveGame|LoadGamefromSlot "CoinValue"))
      (bind _asrunner_save_game (Utilities|Casting|CastToRunner_SaveGame _returnvalue))
      (Variables|Default|SetCoins (Variables|/Game/Runner/Blueprints/Runner_SaveGame.Runner_SaveGame_C|GetCoinsValue _asrunner_save_game)))))

(fn ConstructionScript)

(fn AddFloor
  (bind _returnvalue (Game|SpawnActorfromClass "/Game/Runner/Blueprints/BP_Floor.BP_Floor_C" (Variables|Default|GetFloor%20AttachPoint) "Undefined" "MultiplyWithRoot" 0 0))
  (bind _returnvalue_2 (Default|GetAttachPoint _returnvalue))
  (Variables|Default|SetFloor%20AttachPoint _returnvalue_2)
  (Utilities|Array|Add (Variables|Default|GetFloor%20Tiles) _returnvalue)
  (bind _result (Math|Integer|IncrementInt (Variables|Default|GetFloor%20Count))
    (:%20%20
      (Variables|Default|SetFloor%20Count _result)
      (bind _result_2 (Math|Integer|IncrementInt (Variables|Default|GetFloor%20Count%20For%20Obstacles))
        (:%20%20
          (Variables|Default|SetFloor%20Count%20For%20Obstacles _result_2))))))

(fn ExtendFloor
  (bind _floor_tiles (Variables|Default|GetFloor%20Tiles))
  (bind _output (Utilities|Array|Get(acopy) _floor_tiles))
  (CallFunction|AddFloor)
  (if (> (Utilities|Array|Length (Variables|Default|GetFloor%20Tiles)) (+ (Variables|Default|GetNumberOfTiles) 10))
    (Actor|DestroyActor _output)
    (Utilities|Array|RemoveItem _floor_tiles _output)))

(fn AddEnviroment
  (if (Variables|Default|GetUseOtherEnviro)
    (bind _returnvalue (Game|SpawnActorfromClass "/Game/Runner/Blueprints/BP_Enviroment2.BP_Enviroment2_C" (Variables|Default|GetEnviroment%20Spawn%20Point) "Undefined" "MultiplyWithRoot" 0 0))
    (bind _returnvalue_2 (Default|GetAttachPoint _returnvalue))
    (Variables|Default|SetEnviroment%20Spawn%20Point _returnvalue_2)
    (Utilities|Array|Add (Variables|Default|GetBP_OtherEnviroment) _returnvalue)
    (else
      (bind _returnvalue_3 (Game|SpawnActorfromClass "/Game/Runner/Blueprints/BP_Enviroment.BP_Enviroment_C" (Variables|Default|GetEnviroment%20Spawn%20Point) "Undefined" "MultiplyWithRoot" 0 0))
      (bind _returnvalue_4 (Default|GetAttachPoint _returnvalue_3))
      (Variables|Default|SetEnviroment%20Spawn%20Point _returnvalue_4)
      (Utilities|Array|Add (Variables|Default|GetBP_Enviroment) _returnvalue_3)
      (CallFunction|HandlePortal))))

(fn ExtendEnviroment
  (CallFunction|ExtendEnvironm))

(fn ChangeEnviro
  (params (EnviroSpawn :type Transform))
  (bind _bp_enviroment (Variables|Default|GetBP_Enviroment))
  (Variables|Default|SetEnviroment%20Spawn%20Point EnviroSpawn)
  (Variables|Default|SetUseOtherEnviro true)
  (for _array_element _bp_enviroment
    (Actor|DestroyActor _array_element))
  (Utilities|Array|Clear _bp_enviroment)
  (for _index (range 0 5)
    (CallFunction|AddEnviroment)))

(fn HandlePortal
  (bind _floor_attachpoint (Variables|Default|GetFloor%20AttachPoint))
  (bind _result (Math|Integer|DecrementInt (Variables|Default|GetTilesToChangeEnviro))
    (:%20%20
      (if (and (<= _result 0) (not (Variables|Default|GetPortalSpawned)))
        (Game|SpawnActorfromClass "/Game/Runner/Blueprints/BP_Portal.BP_Portal_C" (Math|Transform|MakeTransform (Math|Vector|MakeVector (.x (.location _floor_attachpoint)) (.y (.location _floor_attachpoint)) 5e+01) (.rotation _floor_attachpoint) "1.000000,1.000000,1.000000") "Undefined" "MultiplyWithRoot" 0 0)
        (Variables|Default|SetPortalSpawned true)))))